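; BP_HealthPack is a timed health pickup that heals BP_Player on overlap with its heart component.
; Below full health it adds health without clamping, plays feedback, calls SpawnHealthPackSPawn on HealthRef, then destroys itself.
; At full health it awards score instead and stays in the world.
; A BeginPlay timer destroys it after a few seconds without calling the spawner.
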(event OnComponentBeginOverlap(StaticMeshComponent)
  (params (OverlappedComponent :type Primitive%20Component%20Object%20Reference) (OtherActor :type Actor%20Object%20Reference) (OtherComp :type Primitive%20Component%20Object%20Reference) (OtherBodyIndex :type Integer) (bFromSweep :type Boolean) (SweepResult :type Hit%20Result%20Structure%20%28by%20ref%29)))

(event OnComponentBeginOverlap(healthpack_BASE_HEART)
  (params (OverlappedComponent :type Primitive%20Component%20Object%20Reference) (OtherActor :type Actor%20Object%20Reference) (OtherComp :type Primitive%20Component%20Object%20Reference) (OtherBodyIndex :type Integer) (bFromSweep :type Boolean) (SweepResult :type Hit%20Result%20Structure%20%28by%20ref%29))
  (bind _asbp_player (Utilities|Casting|CastToBP_Player OtherActor))
  (if (< (Variables|/Game/InfiniteMatrix/Blueprints/BP_Player.BP_Player_C|GetHealth _asbp_player) 100)
    (Development|PrintString "+25 Hp" true false "(R=0.000000,G=0.896269,B=0.000000,A=1.000000)")
    (Variables|/Game/InfiniteMatrix/Blueprints/BP_Player.BP_Player_C|SetHealth _asbp_player (+ (Variables|/Game/InfiniteMatrix/Blueprints/BP_Player.BP_Player_C|GetHealth _asbp_player) 25))
    (Audio|PlaySound2D "/Engine/VREditor/Sounds/UI/Dockable_Window_Open.Dockable_Window_Open" 1.0 1.0 0.0 0 0)
    (Default|SpawnHealthPackSPawn (Variables|Default|GethealthRef))
    (Actor|DestroyActor)
    (else
      (Audio|PlaySound2D "/Engine/VREditor/Sounds/UI/Dockable_Window_Pick_Up.Dockable_Window_Pick_Up" 1.0 1.0 0.0 0 0)
      (Development|PrintString "+10 Score" true true "(R=0.896269,G=0.896269,B=0.896269,A=1.000000)")
      (Variables|/Game/InfiniteMatrix/Blueprints/BP_Player.BP_Player_C|SetScore _asbp_player (+ (Variables|/Game/InfiniteMatrix/Blueprints/BP_Player.BP_Player_C|GetScore _asbp_player) 10)))))

(event EventBeginPlay
  (Utilities|Time|SetTimerbyFunctionName 0 "DestroyHealth" 5.0))

(event EventTick
  (params (DeltaSeconds :type Float%20%28single-precision%29)))

(fn ConstructionScript)

(fn DestroyHealth
  (Actor|DestroyActor))